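; Player character Blueprint with Enhanced Input movement and look, melee attack, health and physics object grabbing.
; Attack plays a push montage whose notify fires a sphere trace to damage pawns, gated until the montage completes.
; Damage lowers health, flashes the HUD, plays a grunt and knocks the player back, or ragdolls at zero health.
; Holding E line-traces from the camera and carries the hit component with a physics handle updated on Tick.
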(event Input|EnhancedActionEvents|EnhancedInputActionMove
  (params (ActionValue :type Vector%202D%20Structure) (ElapsedSeconds :type Float%20%28double-precision%29) (TriggeredSeconds :type Float%20%28double-precision%29) (InputAction :type Input%20Action%20Object%20Reference :default "/Game/Input/Move.Move"))
  (bind _returnvalue (Pawn|GetControlRotation :!class /Script/Engine.Pawn))
  (bind _returnvalue_2 (Pawn|GetControlRotation :!class /Script/Engine.Pawn))
  ;[1 1 1] Movement
  (Pawn|Input|AddMovementInput (Math|Vector|GetRightVector (Math|Rotator|MakeRotator (.roll _returnvalue_2) 0.0 (.yaw _returnvalue_2))) (.x ActionValue) false)
  (Pawn|Input|AddMovementInput (Math|Vector|GetForwardVector (Math|Rotator|MakeRotator (.roll _returnvalue) 0.0 (.yaw _returnvalue))) (.y ActionValue) false))

(event Input|EnhancedActionEvents|EnhancedInputActionLook
  (params (ActionValue :type Vector%202D%20Structure) (ElapsedSeconds :type Float%20%28double-precision%29) (TriggeredSeconds :type Float%20%28double-precision%29) (InputAction :type Input%20Action%20Object%20Reference :default "/Game/Input/Look.Look"))
  ;[1 1 1] Movement
  (Pawn|Input|AddControllerYawInput (.x ActionValue))
  (Pawn|Input|AddControllerPitchInput (* (.y ActionValue) -1.0)))

(event Input|EnhancedActionEvents|EnhancedInputActionAttack
  (params (ActionValue :type Boolean) (ElapsedSeconds :type Float%20%28double-precision%29) (TriggeredSeconds :type Float%20%28double-precision%29) (InputAction :type Input%20Action%20Object%20Reference :default "/Game/Input/Attack.Attack"))
  (bind _attack_trace_pos (Variables|Default|GetAttack%20Trace%20Pos))
  (bind _returnvalue (Transformation|GetWorldLocation _attack_trace_pos))
  ;[1 1 1] Attack
  (:Started
    (if (Variables|Default|GetCan%20Attack)
      (Animation|Montage|PlayMontage (Variables|Character|GetMesh) "/Game/Characters/Mannequins/Animations/Manny/Push_Montage.Push_Montage"
        (:then
          (Variables|Default|SetCan%20Attack false))
        (:OnCompleted
          (Variables|Default|SetCan%20Attack true))
        (:OnNotifyBegin
          (bind (_outhit _returnvalue_2) (Collision|SphereTraceForObjects _returnvalue (+ _returnvalue (* (Math|Vector|GetForwardVector _attack_trace_pos) 1e+02)) 25.0 (Utilities|Array|MakeArray "ObjectTypeQuery3") false 0 "None"))
          (if _returnvalue_2
            (Game|Damage|ApplyDamage (.HitActor (Collision|BreakHitResult _outhit)) 1e+01 0 0)))))))

(event EventBeginPlay
  ;[1 1 1] Input
  (Input|AddMappingContext (PlayerController|LocalPlayerSubsystems|GetEnhancedInputLocalPlayerSubsystem (Game|GetPlayerController 0)) "/Game/Input/Player_Input.Player_Input" 0 "(bIgnoreAllPressedKeysUntilRelease=True,bForceImmediately=False,bNotifyUserSettings=False)")
  (Variables|Default|SetHealth (Variables|Default|GetMax%20Health))
  (bind _returnvalue (UserInterface|CreateWidget "/Game/UI/WB_HealthBar.WB_HealthBar_C"))
  (UserInterface|Viewport|AddtoViewport _returnvalue 0)
  (bind _returnvalue_2 (UserInterface|CreateWidget "/Game/UI/WB_HUD.WB_HUD_C"))
  (bind _output_get (Variables|Default|SetHudWidget _returnvalue_2))
  (UserInterface|Viewport|AddtoViewport _output_get 0))

(event Game|Damage|EventAnyDamage
  (params (Damage :type Float%20%28single-precision%29) (DamageType :type Damage%20Type%20Object%20Reference) (InstigatedBy :type Controller%20Object%20Reference) (DamageCauser :type Actor%20Object%20Reference))
  (Variables|Default|SetHealth (- (Variables|Default|GetHealth) Damage))
  (Default|DamageScreen (Variables|Default|GetHudWidget))
  (Audio|PlaySoundatLocation "/Game/Audio/MS_Danage_Grount.MS_Danage_Grount" (Transformation|GetActorLocation) "0, 0, 0" 1.0 1.0 0.0 0 0 0 0)
  (if (<= (Variables|Default|GetHealth) 0.0)
    (Input|DisableInput 0)
    (Physics|SetSimulatePhysics (Variables|Character|GetMesh) true)
    (else
      (Character|LaunchCharacter (+ (* (Transformation|GetActorForwardVector) -2e+02) (* (Transformation|GetActorUpVector) 1e+02)) false false))))

(event EventTick
  (params (DeltaSeconds :type Float%20%28single-precision%29))
  (bind _camera (Variables|Default|GetCamera))
  ;[1 1 1] Object PíckUp Loop
  (if (Variables|Default|GetIsGrabbing)
    (Physics|Components|PhysicsHandle|SetTargetLocation (Variables|Default|GetPhysicsHandle) (+ (* (Math|Vector|GetForwardVector (Transformation|GetWorldRotation _camera)) 5e+02) (Transformation|GetWorldLocation _camera)))))

(event Input|KeyboardEvents|E
  (params (Key :type Key%20Structure :default "None"))
  (bind _camera (Variables|Default|GetCamera))
  (bind _returnvalue (Transformation|GetWorldLocation _camera))
  ;[1 1 1] Grabbing
  (:Pressed
    (bind (_outhit _returnvalue_2) (Collision|LineTraceByChannel _returnvalue (+ (* (Math|Vector|GetForwardVector (Transformation|GetWorldRotation _camera)) 5e+02) _returnvalue) "TraceTypeQuery1" false 0 "None"))
    (if _returnvalue_2
      (Physics|Components|PhysicsHandle|GrabComponentatLocationwithRotation (Variables|Default|GetPhysicsHandle) (.HitComponent (Collision|BreakHitResult _outhit)) "None" (Transformation|GetWorldLocation (.HitComponent (Collision|BreakHitResult _outhit))) "0, 0, 0")
      (Variables|Default|SetIsGrabbing true)))
  (:Released
    (if (Variables|Default|GetIsGrabbing)
      (Physics|Components|PhysicsHandle|ReleaseComponent (Variables|Default|GetPhysicsHandle))
      (Variables|Default|SetIsGrabbing false))))

(fn ConstructionScript)